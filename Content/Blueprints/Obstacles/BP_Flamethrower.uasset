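; BP_Flamethrower is an obstacle Blueprint whose only logic billboards its Plane component, presumably the flame visual, toward the player's camera.
; Each Tick it casts player 0's character to MainCharacter and takes the horizontal direction from FollowCamera to the Plane.
; That yaw, offset a quarter turn, sets the upright Plane's relative rotation, so it pivots only around the vertical axis.
; The graph contains no damage or overlap logic.
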(event `self.ReceiveTick`
  (params (DeltaSeconds :type "Float (single-precision)"))
  (bind (_returnvalue_x _returnvalue_y) (`KismetMathLibrary.BreakVector` (`SceneComponent.K2_GetComponentLocation` (`self.Plane`))))
  (bind _asmain_character (cast `MainCharacter` (`GameplayStatics.GetPlayerCharacter` 0)))
  (bind (_returnvalue_x_2 _returnvalue_y_2) (`KismetMathLibrary.BreakVector` (`SceneComponent.K2_GetComponentLocation` (`MainCharacter.FollowCamera` _asmain_character))))
  (bind (_returnvalue_roll _returnvalue_pitch _returnvalue_yaw) (`KismetMathLibrary.BreakRotator` (`KismetMathLibrary.MakeRotFromX` (- (`KismetMathLibrary.MakeVector` _returnvalue_x _returnvalue_y) (`KismetMathLibrary.MakeVector` _returnvalue_x_2 _returnvalue_y_2)))))
  (`SceneComponent.K2_SetRelativeRotation` (`self.Plane`) (`KismetMathLibrary.MakeRotator` 90.0 0.0 (+ _returnvalue_yaw 90.0)) false false))

(fn `UserConstructionScript`)